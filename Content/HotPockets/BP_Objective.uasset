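; BP_Objective is an interactable objective that acts as a printer, fridge or water objective, selected by ObjNum.
; When a BP_TaserSphere or BP_DialogueSphere overlaps its Box, it calls the matching Interact function on that sphere's OwningChar.
; It then fires its own matching Printer, Fridge or Water event, all of which are empty here.
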(event `Printer`)

(event `Fridge`)

(event `Water`)

(event `self.Box.OnComponentBeginOverlap`
  (params (OverlappedComponent :type "PrimitiveComponent Object Reference") (OtherActor :type "Actor Object Reference") (OtherComp :type "PrimitiveComponent Object Reference") (OtherBodyIndex :type Integer) (bFromSweep :type Boolean) (SweepResult :type "HitResult Structure (by ref)"))
  (bind _objnum (`self.ObjNum`))
  (bind _asbp_taser_sphere (cast `/Game/HotPockets/BP_TaserSphere` OtherActor)
    (:`then`
      (switch `int` _objnum
        (:`0`
          (bind _owningchar (`/Game/HotPockets/BP_TaserSphere.OwningChar` _asbp_taser_sphere))
          (`/Game/HotPockets/BP_CharacterBase.InteractPrinter` _owningchar)
          (`self.Printer`))
        (:`1`
          (`/Game/HotPockets/BP_CharacterBase.InteractFridge` _owningchar)
          (`self.Fridge`))
        (:`2`
          (`/Game/HotPockets/BP_CharacterBase.InteractWater` _owningchar)
          (`self.Water`))))
    (:`CastFailed`
      (bind _asbp_dialogue_sphere (cast `/Game/HotPockets/BP_DialogueSphere` OtherActor))
      (switch `int` _objnum
        (:`0`
          (bind _owningchar_2 (`/Game/HotPockets/BP_DialogueSphere.OwningChar` _asbp_dialogue_sphere))
          (`/Game/HotPockets/BP_CharacterBase.InteractPrinter` _owningchar_2)
          (`self.Printer`))
        (:`1`
          (`/Game/HotPockets/BP_CharacterBase.InteractFridge` _owningchar_2)
          (`self.Fridge`))
        (:`2`
          (`/Game/HotPockets/BP_CharacterBase.InteractWater` _owningchar_2)
          (`self.Water`))))))

(fn `UserConstructionScript`)