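; BP_WaterCooler is a water cooler actor that launches like a rocket when its Water event is called.
; Water fires once, activating a particle system and enabling physics on the mesh.
; While launched, Tick applies upward velocity-change impulses with slight random sideways jitter.
; A two-second timer ends the thrust, deactivates the particles and spawns an explosion at the mesh, which stays visible.
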(event `self.ReceiveTick`
  (params (DeltaSeconds :type "Float (single-precision)"))
  (if (`self.Rocket`)
    (`PrimitiveComponent.AddImpulse` (`self.StaticMesh1`) (`KismetMathLibrary.MakeVector` (`KismetMathLibrary.RandomFloatInRange` -0.1 0.1) (`KismetMathLibrary.RandomFloatInRange` -0.1 0.1) (`KismetMathLibrary.RandomFloatInRange` 50.0 100.0)) "None" true)
    (`/Engine/EditorBlueprintResources/StandardMacros.DoOnce` false
      (:`Completed`
        (`KismetSystemLibrary.K2_SetTimerDelegate` (delegate `CustomEvent_0`) 2.0)))))

(event `CustomEvent_0`
  (set `self.Rocket` false)
  (`ActorComponent.Deactivate` (`self.ParticleSystem`))
  (`GameplayStatics.SpawnEmitterAtLocation` "/Game/Assets/Particles/P_BRIGHTExplosion.P_BRIGHTExplosion" (`SceneComponent.K2_GetComponentLocation` (`self.StaticMesh1`))))

(event `self.Water`
  (`/Engine/EditorBlueprintResources/StandardMacros.DoOnce` false
    (:`Completed`
      (`ActorComponent.Activate` (`self.ParticleSystem`) false)
      (`PrimitiveComponent.SetSimulatePhysics` (`self.StaticMesh1`) true)
      (set `self.Rocket` true))))

(fn `UserConstructionScript`
  (`parent.UserConstructionScript`))