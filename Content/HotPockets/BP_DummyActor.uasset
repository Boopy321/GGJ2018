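; BP_DummyActor is a dummy with a skeletal mesh that ragdolls and convulses when shocked.
; StartShocking switches the mesh to ragdoll physics, raises a flag and starts a five-second timer that clears it.
; While the flag is set, Tick calls BeenSHOCKED to apply random-direction impulses to the forearm and calf bones every frame.
; The timer ends only the twitching, leaving physics simulation on.
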(event `Been SHOCKED`
  (bind _skeletalmesh (`self.SkeletalMesh`))
  (bind _returnvalue (* (`KismetMathLibrary.RandomUnitVector`) 750.0))
  (`PrimitiveComponent.AddImpulse` _skeletalmesh _returnvalue "lowerarm_l" false)
  (`PrimitiveComponent.AddImpulse` _skeletalmesh _returnvalue "calf_r" false)
  (`PrimitiveComponent.AddImpulse` _skeletalmesh _returnvalue "calf_l" false)
  (`PrimitiveComponent.AddImpulse` _skeletalmesh _returnvalue "lowerarm_r" false))

(event `self.ReceiveTick`
  (params (DeltaSeconds :type "Float (single-precision)"))
  ;[1 1 1] Stops Infinite Loops
  (if (`self.TriggerEventSafely`)
    (`self.Been SHOCKED`)))

(event `StartShocking`
  (bind _skeletalmesh (`self.SkeletalMesh`))
  (`PrimitiveComponent.SetCollisionProfileName` _skeletalmesh "Ragdoll")
  (`PrimitiveComponent.SetSimulatePhysics` _skeletalmesh true)
  (set `self.TriggerEventSafely` true)
  (`KismetSystemLibrary.K2_SetTimerDelegate` (delegate `Reset Taz`) 5.0))

(event `Reset Taz`
  (set `self.TriggerEventSafely` false))

(fn `UserConstructionScript`)