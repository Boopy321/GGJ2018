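; Character base Blueprint that handles NPC conversations and tasing.
; Starting a conversation shows the HUD text and turns the NPC to face the character, while locked movement glides the character toward that NPC.
; Continuing spawns a dialogue sphere, whose collision callback checks the GameInstance dialogue table, then advances the HUD behind a timed cooldown or ends the conversation.
; Tasing spawns a separate taser sphere, and the switch events are empty stubs.
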(event `self.ReceiveBeginPlay`)

(event `self.DeInitConversation`
  (`/Game/HotPockets/WID_Dialogue.SetVisible` (`self.hud`) false))

(event `self.InitConversation`
  (bind _talkingnpc (`self.TalkingNPC`))
  (bind _hud (`self.hud`))
  ;[1 1 1] dunno
  (`/Game/HotPockets/WID_Dialogue.SetVisible` _hud true)
  (`/Game/HotPockets/WID_Dialogue.AdvanceText` _hud _talkingnpc)
  (bind _asbp_npc (cast `/Game/HotPockets/BP_NPC` _talkingnpc))
  (`/Game/HotPockets/BP_NPC.FacePlayer` _asbp_npc (`self.K2_GetActorLocation`)))

(event `self.SetSwitch1`
  ;[1 1 1] change the dial to yes
)

(event `self.SetSwitch2`
  ;[1 1 1] change dial to no
)

(event `self.ReceiveTick`
  (params (DeltaSeconds :type "Float (single-precision)"))
  (bind _returnvalue (`self.K2_GetActorLocation`))
  (bind _returnvalue_2 (`self.K2_GetActorLocation` (`self.TalkingNPC`)))
  (if (`self.bMovementLocked`)
    (if (> (`KismetMathLibrary.VSize` (- _returnvalue_2 _returnvalue)) 120.0)
      (`self.K2_SetActorLocation` (`KismetMathLibrary.VInterpTo_Constant` _returnvalue _returnvalue_2 DeltaSeconds 50.0)))))

(event `self.SetSwitch3`
  ;[1 1 1] change dial goodbye
)

(event `CustomEvent_0`
  (set `self.CanAdvance` true))

(event `DialogueSphereCollide`
  (bind _talkingnpc (`self.TalkingNPC`))
  (`/Engine/EditorBlueprintResources/StandardMacros.IsValid` _talkingnpc
    (:`Is Valid`
      (if (`self.CanAdvance`)
        (bind _asbp_game_instance (cast `/Game/HotPockets/BP_GameInstance` (`GameplayStatics.GetGameInstance`)))
        (bind _outtext (`/Game/HotPockets/BP_GameInstance.GetDialogueFromTable` _asbp_game_instance (`HP_NPC.CharacterID` _talkingnpc) (+ (`HP_NPC.DialogueKey` _talkingnpc) 1)))
        (if (`KismetTextLibrary.NotEqual_TextText` _outtext "")
          (set `self.CanAdvance` false)
          (`KismetSystemLibrary.K2_SetTimerDelegate` (delegate `CustomEvent_0`) 7.0)
          (`/Game/HotPockets/WID_Dialogue.AdvanceText` (`self.hud`) _talkingnpc)
          (else
            (`self.EndConversation`)))))))

(event `self.ContinueConversation`
  ;[1 1 1] advance the text
  (`|SpawnActorFromClass` "/Game/HotPockets/BP_DialogueSphere.BP_DialogueSphere_C" (`KismetMathLibrary.Conv_VectorToTransform` (`SceneComponent.K2_GetComponentLocation` (`self.Scene`))) "Undefined" "OverrideRootScale" null self self))

(event `self.TaserNPC`
  ;[1 1 1] spawn tasersphere
  (`|SpawnActorFromClass` "/Game/HotPockets/BP_TaserSphere.BP_TaserSphere_C" (`KismetMathLibrary.Conv_VectorToTransform` (`SceneComponent.K2_GetComponentLocation` (`self.Scene`))) "Undefined" "OverrideRootScale" null self self))

(fn `UserConstructionScript`)