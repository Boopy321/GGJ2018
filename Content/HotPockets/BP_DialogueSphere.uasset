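; BP_DialogueSphere is a sphere actor tied to an owning first-person character that triggers context interactions on overlap.
; Its overlap event branches on the hit actor: an NPC calls DialogueSphereCollide on the owner, and a door calls Travel.
; Any other actor's component gets a velocity-change impulse along the owner camera's forward direction, shoving it away.
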(event `self.Sphere.OnComponentBeginOverlap`
  (params (OverlappedComponent :type "PrimitiveComponent Object Reference") (OtherActor :type "Actor Object Reference") (OtherComp :type "PrimitiveComponent Object Reference") (OtherBodyIndex :type Integer) (bFromSweep :type Boolean) (SweepResult :type "HitResult Structure (by ref)"))
  (if (!= OtherActor self)
    (cast `/Game/HotPockets/BP_NPC` OtherActor
      (:`then`
        (`/Game/HotPockets/BP_CharacterBase.DialogueSphereCollide` (`self.OwningChar`)))
      (:`CastFailed`
        (bind _asbp_door (cast `/Game/HotPockets/BP_Door` OtherActor)
          (:`then`
            (`/Game/HotPockets/BP_Door.Travel` _asbp_door))
          (:`CastFailed`
            (`PrimitiveComponent.AddImpulse` OtherComp (* (`SceneComponent.GetForwardVector` (`HP_CharacterBase.FirstPersonCameraComponent` (`self.OwningChar`))) 2000.0) "None" true)))))))

(fn `UserConstructionScript`)