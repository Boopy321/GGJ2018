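; BP_NPC is a conversational NPC that faces the player, switches between idle and talking animations, and can be shocked into a ragdoll.
; StartShocking enables ragdoll physics, calls OnShocked, activates lightning and smoke, and sets a five-second flag that makes Tick jolt elbows and knees with random impulses.
; Tick also restarts the idle or talking animation whenever playback stops, following the conversation flag.
; The construction script randomizes each NPC's suit colour.
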(event `Been SHOCKED`
  (bind _charmesh (`self.CharMesh`))
  (bind _returnvalue (* (`KismetMathLibrary.RandomUnitVector`) 750.0))
  (`PrimitiveComponent.AddImpulse` _charmesh _returnvalue "elbow_l" false)
  (`PrimitiveComponent.AddImpulse` _charmesh _returnvalue "knee_r" false)
  (`PrimitiveComponent.AddImpulse` _charmesh _returnvalue "knee_l" false)
  (`PrimitiveComponent.AddImpulse` _charmesh _returnvalue "elbow_r" false))

(event `self.ReceiveTick`
  (params (DeltaSeconds :type "Float (single-precision)"))
  (bind _charmesh (`self.CharMesh`))
  ;[1 1 1] Stops Infinite Loops
  (if (`self.TriggerEventSafely`)
    (`self.Been SHOCKED`))
  (if (`SkeletalMeshComponent.IsPlaying` (`self.CharMesh`))
    _
    (elif (`self.Talking`)
      (`SkeletalMeshComponent.PlayAnimation` _charmesh "/Game/Assets/Skeltons/Animations/Mike_Talking_Anim.Mike_Talking_Anim" false)
      (else
        (`SkeletalMeshComponent.PlayAnimation` _charmesh "/Game/Assets/Skeltons/Animations/Mike_Idle_Anim.Mike_Idle_Anim" false)))))

(event `StartShocking`
  (bind _charmesh (`self.CharMesh`))
  (`PrimitiveComponent.SetCollisionProfileName` _charmesh "Ragdoll")
  (`PrimitiveComponent.SetSimulatePhysics` _charmesh true)
  (set `self.TriggerEventSafely` true)
  (`KismetSystemLibrary.K2_SetTimerDelegate` (delegate `Reset Taz`) 5.0)
  (`self.OnShocked`)
  (`ActorComponent.Activate` (`self.Lightning`) true)
  (`ActorComponent.Activate` (`self.Smoke`) false))

(event `Reset Taz`
  (set `self.TriggerEventSafely` false))

(event `FacePlayer`
  (params (PlayerPos :type "Vector Structure"))
  (bind (_returnvalue_roll _returnvalue_pitch _returnvalue_yaw) (`KismetMathLibrary.BreakRotator` (`KismetMathLibrary.FindLookAtRotation` (`self.K2_GetActorLocation`) PlayerPos)))
  (`self.K2_SetActorRotation` (`KismetMathLibrary.MakeRotator` _returnvalue_roll 0.0 (+ _returnvalue_yaw 270.0))))

(event `Recoil`
  (`SkeletalMeshComponent.PlayAnimation` (`self.CharMesh`) "/Game/Assets/Skeltons/Animations/Mike_Zapped.Mike_Zapped" false))

(event `Converse`
  (`SkeletalMeshComponent.PlayAnimation` (`self.CharMesh`) "/Game/Assets/Skeltons/Animations/Mike_Talking_Anim.Mike_Talking_Anim" false))

(event `BeginConvo`
  (set `self.Talking` true))

(event `EndConvo`
  (set `self.Talking` false))

(fn `UserConstructionScript`
  (`MeshComponent.SetVectorParameterValueOnMaterials` (`self.CharMesh`) "Suit Colour" (`KismetMathLibrary.MakeVector` (`KismetMathLibrary.RandomFloatInRange` 0.5 0.7) (`KismetMathLibrary.RandomFloatInRange` 0.5 0.7) (`KismetMathLibrary.RandomFloatInRange` 0.5 0.7))))