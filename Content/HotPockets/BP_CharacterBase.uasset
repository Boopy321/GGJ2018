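; BP_CharacterBase is a character Blueprint that runs NPC conversations and a taser action.
; Conversation init and deinit toggle the HUD, with init also advancing the TalkingNPC's text.
; Continue and taser actions spawn sphere actors owned by the character.
; DialogueSphereCollide looks up the NPC's next line through BP_GameInstance, advancing the HUD or ending the conversation when it is empty; dial switch events are empty stubs.
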(event `self.ReceiveBeginPlay`)

(event `self.DeInitConversation`
  (`/Game/HotPockets/WID_Dialogue.SetVisible` (`self.hud`) false))

(event `self.InitConversation`
  (bind _hud (`self.hud`))
  ;[1 1 1] dunno
  (`/Game/HotPockets/WID_Dialogue.SetVisible` _hud true)
  (`/Game/HotPockets/WID_Dialogue.AdvanceText` _hud (`self.TalkingNPC`)))

(event `self.SetSwitch1`
  ;[1 1 1] change the dial to yes
)

(event `self.SetSwitch2`
  ;[1 1 1] change dial to no
)

(event `self.SetSwitch3`
  ;[1 1 1] change dial goodbye
)

(event `DialogueSphereCollide`
  (bind _talkingnpc (`self.TalkingNPC`))
  (`/Engine/EditorBlueprintResources/StandardMacros.IsValid` _talkingnpc
    (:`Is Valid`
      (bind _asbp_game_instance (cast `/Game/HotPockets/BP_GameInstance` (`GameplayStatics.GetGameInstance`)))
      (bind _outtext (`/Game/HotPockets/BP_GameInstance.GetDialogueFromTable` _asbp_game_instance (`HP_NPC.CharacterID` _talkingnpc) (+ (`HP_NPC.DialogueKey` _talkingnpc) 1)))
      (if (`KismetTextLibrary.NotEqual_TextText` _outtext "")
        (`/Game/HotPockets/WID_Dialogue.AdvanceText` (`self.hud`) _talkingnpc)
        (else
          (`self.EndConversation`))))))

(event `self.ContinueConversation`
  ;[1 1 1] advance the text
  (`|SpawnActorFromClass` "/Game/HotPockets/BP_DialogueSphere.BP_DialogueSphere_C" (`KismetMathLibrary.Conv_VectorToTransform` (`SceneComponent.K2_GetComponentLocation` (`self.Scene`))) "Undefined" "OverrideRootScale" null self self))

(event `self.TaserNPC`
  ;[1 1 1] spawn tasersphere
  (`|SpawnActorFromClass` "/Game/HotPockets/BP_TaserSphere.BP_TaserSphere_C" (`KismetMathLibrary.Conv_VectorToTransform` (`SceneComponent.K2_GetComponentLocation` (`self.Scene`))) "Undefined" "OverrideRootScale" null self self))

(fn `UserConstructionScript`)